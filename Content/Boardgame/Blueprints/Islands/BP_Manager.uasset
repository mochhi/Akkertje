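; Board game manager that moves the player (BP_Speler) along zone routes by dice roll.
; On BeginPlay it sorts board tiles into per-zone arrays by TileIndex and creates the dice and zone-choice widgets.
; Choosing a zone or route resets the tile index and teleports the player to its first tile.
; A 1–4 roll computes a target index, checks it against route length, then looks up the tile for teleporting.
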(event `self.ReceiveBeginPlay`
  (bind _returnvalue (`GameplayStatics.GetActorOfClass` "/Game/Boardgame/Blueprints/Islands/BP_Speler.BP_Speler_C"))
  (set `self.Ref Speler` _returnvalue)
  (`self.BuildRouteArrays`)
  (bind _returnvalue_2 (`|CreateWidget` "/Game/Boardgame/Blueprints/Islands/WBP_Dobbel.WBP_Dobbel_C"))
  (bind _output_get (set `self.Ref DobbelWidget` _returnvalue_2))
  (`UserWidget.AddToViewport` _output_get 0)
  (bind _returnvalue_3 (`|CreateWidget` "/Game/Boardgame/Blueprints/Islands/WBP_ZoneChoice.WBP_ZoneChoice_C"))
  (bind _output_get_2 (set `self.Ref ZoneChoice` _returnvalue_3))
  (`UserWidget.AddToViewport` _output_get_2 0))

(event `OnZoneChosenBeforeRoll`
  (params (NewZone :type "/Game/Boardgame/Blueprints/Enum/E_TypeWeg Enum" :default "NewEnumerator0"))
  (bind _output_get (set `self.ChosenZone` NewZone))
  (set `self.CurrentTileIndex` 0)
  (set `self.OverflowSteps` 0)
  (set `self.StepsRemaining` 0)
  (bind (_outtile _tileexists _teleporttilelocation) (`self.GetTileIndexFromZone` _output_get))
  (if _tileexists
    (`/Game/Boardgame/Blueprints/Islands/BP_Speler.TeleportToBoardLocation` (`self.Ref Speler`) _teleporttilelocation)))

(fn `BuildRouteArrays`
  (bind _outactors (`GameplayStatics.GetAllActorsOfClass` "/Game/Boardgame/Blueprints/BP_BoardTileMain.BP_BoardTileMain_C"))
  (for _array_element _outactors
    (bind _asbp_board_tile_main (cast `/Game/Boardgame/Blueprints/BP_BoardTileMain` _array_element))
    (switch `/Game/Boardgame/Blueprints/Enum/E_TypeWeg` (`/Game/Boardgame/Blueprints/BP_BoardTileMain.Type Weg` _array_element)
      (:`NewEnumerator0`
        (bind _tileindex (`/Game/Boardgame/Blueprints/BP_BoardTileMain.TileIndex` _array_element))
        (`KismetArrayLibrary.Array_Set` (`self.Y_Risky`) _tileindex _asbp_board_tile_main true))
      (:`NewEnumerator1`
        (`KismetArrayLibrary.Array_Set` (`self.Y_Safe`) _tileindex _asbp_board_tile_main true))
      (:`NewEnumerator2`
        (`KismetArrayLibrary.Array_Set` (`self.Y_Shortcut`) _tileindex _asbp_board_tile_main true))
      (:`NewEnumerator3`
        (`KismetArrayLibrary.Array_Set` (`self.Y_SafeZoneNormal`) _tileindex _asbp_board_tile_main true))
      (:`NewEnumerator4`
        (`KismetArrayLibrary.Array_Set` (`self.Y_SafeZoneArtifact`) _tileindex _asbp_board_tile_main true)))))

(fn `DiceRoll`
  (bind _output_get (set `self.OutputDiceRoll` (`KismetMathLibrary.RandomIntegerInRange` 1 4)))
  (`KismetSystemLibrary.PrintString` (`KismetStringLibrary.Conv_IntToString` _output_get))
  (`self.HandleDiceRollMove` _output_get))

(fn `GetTileIndexFromZone`
  (params (ChosenZone :type "/Game/Boardgame/Blueprints/Enum/E_TypeWeg Enum" :default "NewEnumerator0") (WantedTileIndex :type Integer))
  (returns (OutTile :type "/Game/Boardgame/Blueprints/BP_BoardTileMain Object Reference") (TileExists :type Boolean) (TeleportTileLocation :type "Vector Structure"))
  (locals (SelectedRouteArray :type "Array of /Game/Boardgame/Blueprints/BP_BoardTileMain Object Reference"))
  (switch `/Game/Boardgame/Blueprints/Enum/E_TypeWeg` ChosenZone
    (:`NewEnumerator0`
      (bind _output_get (set `local.SelectedRouteArray` (`self.Y_Risky`)))
      (if (`KismetArrayLibrary.Array_IsValidIndex` _output_get WantedTileIndex)
        (bind _output (`|GetArrayItem` _output_get WantedTileIndex))
        (return _output true (`self.K2_GetActorLocation` _output))))
    (:`NewEnumerator1`
      (bind _output_get_2 (set `local.SelectedRouteArray` (`self.Y_Safe`)))
      (bind _output_2 (`|GetArrayItem` _output_get_2 WantedTileIndex))
      (return _output_2 true (`self.K2_GetActorLocation` _output_2)))
    (:`NewEnumerator2`
      (bind _output_get_3 (set `local.SelectedRouteArray` (`self.Y_Shortcut`)))
      (bind _output_3 (`|GetArrayItem` _output_get_3 WantedTileIndex))
      (return _output_3 true (`self.K2_GetActorLocation` _output_3)))
    (:`NewEnumerator3`
      (bind _output_get_4 (set `local.SelectedRouteArray` (`self.Y_SafeZoneNormal`)))
      (bind _output_4 (`|GetArrayItem` _output_get_4 WantedTileIndex))
      (return _output_4 true (`self.K2_GetActorLocation` _output_4)))
    (:`NewEnumerator4`
      (bind _output_get_5 (set `local.SelectedRouteArray` (`self.Y_SafeZoneNormal`)))
      (bind _output_5 (`|GetArrayItem` _output_get_5 WantedTileIndex))
      (return _output_5 true (`self.K2_GetActorLocation` _output_5)))))

(fn `GetZoneLength`
  (params (ChosenZone :type "/Game/Boardgame/Blueprints/Enum/E_TypeWeg Enum" :default "NewEnumerator0"))
  (returns (RouteLength :type Integer))
  (switch `/Game/Boardgame/Blueprints/Enum/E_TypeWeg` ChosenZone
    (:`NewEnumerator0`
      (return (`KismetArrayLibrary.Array_Length` (`self.Y_Risky`))))
    (:`NewEnumerator1`
      (return (`KismetArrayLibrary.Array_Length` (`self.Y_Safe`))))
    (:`NewEnumerator2`
      (return (`KismetArrayLibrary.Array_Length` (`self.Y_Shortcut`))))
    (:`NewEnumerator3`
      (return (`KismetArrayLibrary.Array_Length` (`self.Y_SafeZoneNormal`))))
    (:`NewEnumerator4`
      (return (`KismetArrayLibrary.Array_Length` (`self.Y_SafeZoneArtifact`))))))

(fn `HandleDiceRollMove`
  (params (RolledValue :type Integer))
  (bind _output_get (set `self.StepsRemaining` RolledValue))
  (bind _output_get_2 (set `self.WantedTileIndex` (+ _output_get (`self.CurrentTileIndex`))))
  (bind _routelength (`self.GetZoneLength` (`self.ChosenZone`)))
  (bind _output_get_3 (set `self.RouteLength` _routelength))
  (bind _output_get_4 (set `self.LastValidIndex` (- _output_get_3 1)))
  (if (<= _output_get_4 _output_get_2)
    (bind (_outtile _tileexists _teleporttilelocation) (`self.GetTileIndexFromZone` (`self.ChosenZone`) _output_get_2))
    (if _tileexists
      (set `self.CurrentTileIndex` (`self.WantedTileIndex`))
      (set `self.StepsRemaining` 0)
      (`/Game/Boardgame/Blueprints/Islands/BP_Speler.TeleportToBoardLocation` (`self.Ref Speler`) _teleporttilelocation))))

(fn `NewFunction`)

(fn `OnRouteChosen`
  (params (NewRoute :type "/Game/Boardgame/Blueprints/Enum/E_TypeWeg Enum" :default "NewEnumerator0"))
  (set `self.ChosenZone` NewRoute)
  (set `self.CurrentTileIndex` 0)
  (bind (_outtile _tileexists _teleporttilelocation) (`self.GetTileIndexFromZone` NewRoute))
  (if _tileexists
    (`/Game/Boardgame/Blueprints/Islands/BP_Speler.TeleportToBoardLocation` (`self.Ref Speler`) _teleporttilelocation)
    (bind _output_get (set `self.OverflowSteps` (- (`self.OverflowSteps`) 0)))
    (if (> _output_get 0)
      (`self.HandleDiceRollMove` _output_get))))

(fn `SetDiceVisible`
  (params (IsVisible :type Boolean)))

(fn `UserConstructionScript`)