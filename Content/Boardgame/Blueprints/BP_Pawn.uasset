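; Board game pawn that advances along indexed tiles by dice roll, teleporting to locations supplied by BP_GameflowManager.
; ContinueMove recurses per step, signalling the final tile or pausing at zone ends to save leftover steps and show map selection.
; OnZoneChosen relocates the pawn, then triggers mid-island handling or restores leftover steps without clearing the wait flag that blocks ContinueMove.
; GoNextZoneEndIndex's search logic is disconnected, leaving the dice overflow pre-split inactive.
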(event `self.ReceiveBeginPlay`
  (bind _returnvalue (`GameplayStatics.GetActorOfClass` "/Game/Boardgame/Blueprints/BP_GameflowManager.BP_GameflowManager_C"))
  (set `self.BP_GameflowManager_Ref` _returnvalue)
  (set `self.CurrentTileIndex` (`self.StartTileIndex`)))

(event `OnZoneChosen`
  (params (ChosenStartIndex :type Integer))
  (bind _output_get (set `self.CurrentTileIndex` ChosenStartIndex))
  (bind _location (`/Game/Boardgame/Blueprints/BP_GameflowManager.GetTileLocationByIndex` (`self.BP_GameflowManager_Ref`) _output_get))
  (`self.K2_SetActorLocation` _location false true)
  (if (`self.bChoosingZoneAfterShop`)
    (`self.OnMidIslandRouteChose`)
    (else
      (set `self.bWaitingForZoneChoice` (`self.bWaitingForZoneChoice`))
      (set `self.bIsMoving` true)
      (set `self.StepsRemaining` (`self.OverflowSteps`))
      (set `self.OverflowSteps` 0)
      (`self.ContinueMove`))))

(fn `ContinueMove`
  (bind _stepsremaining (`self.StepsRemaining`))
  (if (`self.bWaitingForZoneChoice`)
    (return)
    (elif (<= (`self.StepsRemaining`) 0)
      (set `self.bIsMoving` false)
      (return)
      (else
        (bind _output_get (set `self.TargetTileIndex` (+ (`self.CurrentTileIndex`) 1)))
        (bind _location (`/Game/Boardgame/Blueprints/BP_GameflowManager.GetTileLocationByIndex` (`self.BP_GameflowManager_Ref`) _output_get))
        (`self.K2_SetActorLocation` _location false true)
        (set `self.CurrentTileIndex` (`self.TargetTileIndex`))
        (set `self.StepsRemaining` (- (`self.StepsRemaining`) 1))
        (if (`KismetArrayLibrary.Array_Contains` (`self.ZoneEndIndexNumbers`) (`self.CurrentTileIndex`))
          (set `self.OverflowSteps` _stepsremaining)
          (set `self.StepsRemaining` 0)
          (set `self.bIsMoving` false)
          (set `self.bWaitingForZoneChoice` true)
          (`/Game/Boardgame/Blueprints/BP_GameflowManager.ShowMapSelectionWidget` (`self.BP_GameflowManager_Ref`))
          (return)
          (elif (> _stepsremaining 0)
            (`self.ContinueMove`)
            (else
              (set `self.bIsMoving` false)
              (`self.PawnReachedFinalTile` (`self.CurrentTileIndex`))
              (return))))))))

(fn `GoNextZoneEndIndex`
  (params (FromIndex :type Integer))
  (returns (NextZoneEndIndex :type Integer) (bFound :type Boolean)))

(fn `OnMidIslandRouteChose`
  (set `self.bWaitingForZoneChoice` false)
  (set `self.bIsMoving` false)
  (set `self.StepsRemaining` 0)
  (set `self.OverflowSteps` 0)
  (set `self.bChoosingZoneAfterShop` true)
  (`/Game/Boardgame/Blueprints/BP_GameflowManager.HandleArrivedMidIsland` (`self.BP_GameflowManager_Ref`)))

(fn `StartMoveFromDice`
  (params (DiceValue :type Integer))
  (bind _returnvalue (- (`self.NextZoneEndIndex`) (`self.CurrentTileIndex`)))
  (set `self.bWaitingForZoneChoice` false)
  (set `self.OverflowSteps` 0)
  (set `self.StepsRemaining` DiceValue)
  (bind (_nextzoneendindex _bfound) (`self.GoNextZoneEndIndex` (`self.CurrentTileIndex`)))
  (if _bfound
    (if (> DiceValue _returnvalue)
      (set `self.OverflowSteps` (- DiceValue _returnvalue))
      (set `self.StepsRemaining` _returnvalue)
      (`self.ContinueMove` :!label _label))
    (else
      (goto _label))))

(fn `UserConstructionScript`)