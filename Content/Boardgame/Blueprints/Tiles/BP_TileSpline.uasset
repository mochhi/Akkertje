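; Board game path actor that lays the level's BP_BoardTile actors along its spline.
; UpdateTiles gathers every tile with GetAllActorsOfClass, then DistributeTilesOnSpline numbers each by array order and moves it to a fixed-spacing distance, setting location only.
; It runs on construction, BeginPlay and the UpdateTilesInEditor event.
; Disconnected leftovers hold earlier spawn, child-actor and instanced-mesh approaches.
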(event `self.ReceiveBeginPlay`
  (`self.UpdateTiles`))

(event `DistributeTilesOnSpline`
  (set `self.Tile Count` (`KismetArrayLibrary.Array_Length` (`self.PLS`)))
  (if (> (`self.Tile Count`) 0)
    (for (_array_element _array_index) (`self.PLS`)
      (set `/Game/Boardgame/Blueprints/BP_BoardTileMain.TileIndex` _array_index _array_element)
      (`self.K2_SetActorLocation` _array_element (`SplineComponent.GetLocationAtDistanceAlongSpline` (`self.Tile Spline`) (* _array_index (`self.Spacing`)) "World") false false))))

(event `UpdateTilesInEditor`
  (`self.UpdateTiles`))

(fn `Update Spawn Tiles`
  (for _index (range (+ (- (`KismetArrayLibrary.Array_Length` (`self.Spawned Tiles`)) -1) 1))
    (bind _output (`|GetArrayItem` (`self.Spawned Tiles`) _index))
    (if (`KismetSystemLibrary.IsValid` _output)
      (`self.K2_SetActorTransform` _output (`SplineComponent.GetTransformAtDistanceAlongSpline` (`self.Tile Spline`) (* _index (`self.Spacing`)) "World" false) false false))))

(fn `UpdateTiles`
  (bind _outactors (`GameplayStatics.GetAllActorsOfClass` "/Game/Boardgame/Blueprints/BP_BoardTile.BP_BoardTile_C"))
  (set `self.PLS` _outactors)
  (`self.DistributeTilesOnSpline`))

(fn `UserConstructionScript`
  (`self.UpdateTiles`))