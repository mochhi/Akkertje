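; BP_BoardTile is a board game tile with a mesh, an index and a text label, but all of its logic is currently disconnected.
; Unwired construction script nodes would set TileIndex to the last index of all placed BP_BoardTile actors and display it as text.
; An unwired ColorSwitch body would pick a branch by TileIndex modulo four to set the tile's overlay material, though no materials are shown.
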(fn `Color Switch`)

(fn `UserConstructionScript`)