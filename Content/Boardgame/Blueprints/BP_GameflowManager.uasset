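; Gameflow manager for a board game, running the round loop of dice roll, pawn movement and category assignment.
; On BeginPlay it caches pawn and UI references, creates dice, confirm and score widgets, and sorts tiles by index.
; Rolls move the pawn, whose final tile selects the category widget (only Lijntje connected); closing the assignment restores the dice.
; Helpers provide tile locations, difficulty points, score broadcasts and the mid-island shop button.
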(event `self.ReceiveBeginPlay`
  ; Find all refrences
  (`self.Create Class Refrences`)
  (`self.Create Widget Refrences`)
  (`self.Call Widget & Button event`)
  (`self.Sorting Index Tiles`))

(event `Call Widget & Button event`
  ; Initiate Category widget
  (add `/Game/Boardgame/Blueprints/BP_Pawn.PawnReachedFinalTile` (`self.REF_Pawn`) (delegate `OpeningWidget`))
  ; Set dice button visible
  (add `/Game/Boardgame/Blueprints/Widgets/WBP_ConfirmPage.OnAssignmentClosed` (`self.REF_ConfirmpageRef`) (delegate `ResetRound`))
  (`self.SetDiceVisible` true))

(event `ResetRound`
  ; Set dice button visible
  (`self.SetDiceVisible` true))

(event `OpeningWidget`
  (params (FinalTileIndex :type Integer))
  ; Initiate Category widget
  (`self.OpenCategoryWidget` (`/Game/Boardgame/Blueprints/BP_BoardTileMain.Category_0` (`|GetArrayItem` (`self.Tiles`) FinalTileIndex))))

(fn `Create Class Refrences`
  (`|ExecutionSequence`
    (:`then_0`
      (bind _returnvalue (`GameplayStatics.GetActorOfClass` "/Game/Boardgame/Blueprints/BP_Pawn.BP_Pawn_C"))
      (set `self.REF_Pawn` _returnvalue))
    (:`then_1`
      (bind _returnvalue_2 (`GameplayStatics.GetActorOfClass` "/Game/Boardgame/Blueprints/User_Interface/BP_UserInterface.BP_UserInterface_C"))
      (set `self.REF_UserInterface` _returnvalue_2))))

(fn `Create Widget Refrences`
  (`|ExecutionSequence`
    (:`then_0`
      (bind _returnvalue (`|CreateWidget` "/Game/Boardgame/Blueprints/Widgets/WBP_DiceButton.WBP_DiceButton_C"))
      (bind _output_get (set `self.REF_Dice` _returnvalue))
      (`UserWidget.AddToViewport` _output_get 0)
      (`Widget.SetVisibility` _output_get "Collapsed"))
    (:`then_1`
      (bind _returnvalue_2 (`|CreateWidget` "/Game/Boardgame/Blueprints/Widgets/WBP_ConfirmPage.WBP_ConfirmPage_C"))
      (bind _output_get_2 (set `self.REF_ConfirmpageRef` _returnvalue_2))
      (`UserWidget.AddToViewport` _output_get_2 0)
      (`Widget.SetVisibility` _output_get_2 "Collapsed"))
    (:`then_2`
      (bind _returnvalue_3 (`|CreateWidget` "/Game/Boardgame/Blueprints/Widgets/WBP_TotalScore.WBP_TotalScore_C"))
      (bind _output_get_3 (set `self.REF_Score` _returnvalue_3))
      (`UserWidget.AddToViewport` _output_get_3 0))))

(fn `DiceRoll`
  (bind _output_get (set `self.OutputDiceRoll` (`KismetMathLibrary.RandomIntegerInRange` 1 6)))
  (`KismetSystemLibrary.PrintString` (`KismetStringLibrary.Conv_IntToString` _output_get))
  (`/Game/Boardgame/Blueprints/BP_Pawn.StartMoveFromDice` (`self.REF_Pawn`) _output_get)
  (`self.SetDiceVisible` false))

(fn `GetPointsFromDifficulty`
  (params (Difficulty :type Integer))
  (returns (Points :type Integer))
  (switch `int` Difficulty
    (:`0`
      (return 1))
    (:`1`
      (return 3))
    (:`2`
      (return 5))))

(fn `GetTileLocationByIndex`
  (params (TileIndex :type Integer))
  (returns (Location :type "Vector Structure"))
  (locals (`Tile Length` :type Integer :default 0) (`Tile Index` :type Integer))
  (bind _tile_index (`local.Tile Index`))
  (bind _output (`|GetArrayItem` (`self.Tiles`) (`local.Tile Index`)))
  (set `local.Tile Index` TileIndex)
  (set `local.Tile Length` (`KismetArrayLibrary.Array_Length` (`self.Tiles`)))
  (if (> (`local.Tile Length`) (`local.Tile Index`))
    (if (and (< _tile_index (`local.Tile Length`)) (>= _tile_index 0))
      (if (`KismetSystemLibrary.IsValid` _output)
        (return (`self.K2_GetActorLocation` _output))
        (else
          (return (0.0 0.0 0.0))))
      (else
        (return (0.0 0.0 0.0))))
    (else
      (return (0.0 0.0 0.0)))))

(fn `HandleArrivedMidIsland`
  (`/Game/Boardgame/Blueprints/User_Interface/BP_UserInterface.Shop Button` (`self.REF_UserInterface`) true))

(fn `OpenCategoryWidget`
  (params (Category :type "/Game/Boardgame/Blueprints/User_Interface/E_Category Enum" :default "NewEnumerator0"))
  (switch `/Game/Boardgame/Blueprints/User_Interface/E_Category` Category
    (:`NewEnumerator0`
      (bind _returnvalue (`|CreateWidget` "/Game/Boardgame/Blueprints/Widgets/WBP_Lijntje.WBP_Lijntje_C"))
      (`UserWidget.AddToViewport` _returnvalue 0))))

(fn `SetDiceVisible`
  (params (IsVisible :type Boolean))
  (bind _ref_dice (`self.REF_Dice`))
  (if (`KismetSystemLibrary.IsValid` _ref_dice)
    (if IsVisible
      (`Widget.SetVisibility` _ref_dice "Visible")
      (else
        (`Widget.SetVisibility` _ref_dice "Collapsed")))))

(fn `SetTotalUpdatedScore`
  (params (NewScore :type Integer))
  (bind _output_get (set `self.TotalPoints` NewScore))
  (`self.OnScoreUpdated` _output_get))

(fn `ShowConfirmationScreen`
  (params (IsVisible :type Boolean))
  (bind _ref_confirmpageref (`self.REF_ConfirmpageRef`))
  (if IsVisible
    (`Widget.SetVisibility` _ref_confirmpageref "Visible")
    (else
      (`Widget.SetVisibility` _ref_confirmpageref "Collapsed"))))

(fn `Sorting Index Tiles`
  (bind _outactors (`GameplayStatics.GetAllActorsOfClass` "/Game/Boardgame/Blueprints/BP_BoardTileMain.BP_BoardTileMain_C"))
  (for _array_element _outactors
    (`KismetArrayLibrary.Array_Set` (`self.Tiles`) (`/Game/Boardgame/Blueprints/BP_BoardTileMain.TileIndex` _array_element) _array_element true)))

(fn `UserConstructionScript`)